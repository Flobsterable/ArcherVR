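; BP_Arro is a projectile actor, apparently a VR bow arrow, that motion controllers pick up and drop.
; Pickup attaches the mesh to the hand, snapping to the socket when very close, while Drop detaches it only without a valid bow reference.
; Shoot activates ProjectileMovement at the given local forward velocity, and a sphere overlap halts it while flagged as flying.
; The construction script disables mesh physics.
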(event OnComponentBeginOverlap(Sphere)
  (params (OverlappedComponent :type Primitive%20Component%20Object%20Reference) (OtherActor :type Actor%20Object%20Reference) (OtherComp :type Primitive%20Component%20Object%20Reference) (OtherBodyIndex :type Integer) (bFromSweep :type Boolean) (SweepResult :type Hit%20Result%20Structure%20%28by%20ref%29))
  (bind _projectilemovement (Variables|Default|GetProjectileMovement))
  (if (Variables|Default|GetIsFly?)
    (Components|Movement|StopMovementImmediately _projectilemovement)
    (Components|Activation|SetActive _projectilemovement false false)))

(event Custom|Shoot
  (params (Velocity :type Float%20%28single-precision%29))
  (bind _projectilemovement (Variables|Default|GetProjectileMovement))
  (Variables|/Script/Engine.ProjectileMovementComponent|SetInitialSpeed _projectilemovement Velocity)
  (Variables|/Script/Engine.ProjectileMovementComponent|SetMaxSpeed _projectilemovement Velocity)
  (Game|Components|ProjectileMovement|SetVelocityinLocalSpace _projectilemovement (Math|Vector|MakeVector Velocity 0.0 0.0))
  (Components|Activation|SetActive (Variables|Default|GetProjectileMovement) true false))

(event EventPickup
  (params (AttachTo :type Scene%20Component%20Object%20Reference) (HandMesh :type Scene%20Component%20Object%20Reference))
  (if (< (Math|Vector|VectorLength (- (Transformation|GetWorldLocation (Variables|Default|GetStaticMesh)) (Transformation|GetSocketLocation HandMesh "hand_Socket"))) 5.0)
    (Transformation|AttachComponentToComponent (Variables|Default|GetStaticMesh) HandMesh "hand_Socket" "SnapToTarget" "SnapToTarget" "KeepWorld" false)
    (else
      (Transformation|AttachComponentToComponent (Variables|Default|GetStaticMesh) HandMesh "None" "KeepWorld" "KeepWorld" "KeepWorld" false))))

(event EventDrop
  (params (HandMesh :type Scene%20Component%20Object%20Reference) (MotionController :type Scene%20Component%20Object%20Reference))
  (Utilities|IsValid (Variables|Default|GetBow_Ref)
    (:Is%20Not%20Valid
      (Transformation|DetachFromComponent (Variables|Default|GetStaticMesh) "KeepWorld" "KeepWorld" "KeepWorld" true))))

(fn ConstructionScript
  (Physics|SetSimulatePhysics (Variables|Default|GetStaticMesh) false))