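; Two-handed VR bow that motion controllers pick up, draw and release to fire arrows.
; The first hand holds the bow; a second pickup, gated by the first hand's distance to the string socket, spawns an arrow on the string.
; Tick aims the bow along the line between both hands.
; Releasing the second hand fires, with power from curve-remapped draw distance; releasing the first restores physics.
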(event OnComponentBeginOverlap(Sphere)
  (params (OverlappedComponent :type Primitive%20Component%20Object%20Reference) (OtherActor :type Actor%20Object%20Reference) (OtherComp :type Primitive%20Component%20Object%20Reference) (OtherBodyIndex :type Integer) (bFromSweep :type Boolean) (SweepResult :type Hit%20Result%20Structure%20%28by%20ref%29)))

(event Custom|SpawnArrow
  (bind _returnvalue (Game|SpawnActorfromClass "/Game/Blueprints/BP_Arro.BP_Arro_C" (Math|Transform|MakeTransform "0, 0, 0") "AlwaysSpawn" 0 0))
  (bind _output_get (Variables|Default|SetArrow _returnvalue))
  (Transformation|AttachComponentToComponent _output_get (Variables|Default|GetSkeletalMesh) "bowString" "SnapToTarget" "SnapToTarget" "KeepWorld" false)
  (Development|PrintString "Hello")
  (Transformation|SetActorRotation (Variables|Default|GetArrow) (Transformation|GetWorldRotation (Variables|Default|GetSphere))))

(event Custom|Shoot
  (Transformation|DetachFromActor (Variables|Default|GetArrow) "KeepWorld" "KeepWorld" "KeepRelative")
  (Default|Shoot (Variables|Default|GetArrow) (Math|Float|MapRangeClamped (Math|Float|Clamp(Float) (Math|Curves|GetFloatValue (Variables|Default|GetFloatCurve) (- (CallFunction|GetDistanceHands) (Variables|Default|GetDistFault))) 0.0 6e+01) 0.0 1.0 6e+01 2e+03))
  (Variables|Default|SetArrow 0))

(event EventTick
  (params (DeltaSeconds :type Float%20%28single-precision%29))
  (Utilities|FlowControl|Sequence
    (:then_0
      (Utilities|IsValid (Variables|Default|GetFirstMotion)
        (:Is%20Valid
          (Utilities|IsValid (Variables|Default|GetSecondMontion)
            (:Is%20Valid
              (Transformation|SetActorRotation (Class|KismetMathLibrary|MakeRotfromYX (- (Transformation|GetSocketLocation (Variables|Default|GetFirstHand%20Mesh) "hand_Socket") (Transformation|GetWorldLocation (Variables|Default|GetSecondHand%20Mesh))) (Math|Vector|GetUpVector (Variables|Default|GetFirstHand%20Mesh)))))))))))

(event EventPickup
  (params (AttachTo :type Scene%20Component%20Object%20Reference) (HandMesh :type Scene%20Component%20Object%20Reference))
  (Utilities|IsValid (Variables|Default|GetFirstMotion)
    (:Is%20Valid
      (if (< (Math|Vector|VectorLength (- (Transformation|GetSocketLocation (Variables|Default|GetSkeletalMesh) "bowString") (Transformation|GetWorldLocation (Variables|Default|GetFirstHand%20Mesh)))) 1e+01)
        (Variables|Default|SetSecondMontion AttachTo)
        (Variables|Default|SetSecondHand%20Mesh HandMesh)
        (CallFunction|SpawnArrow)
        (Variables|Default|SetDistFault (CallFunction|GetDistanceHands))))
    (:Is%20Not%20Valid
      (Variables|Default|SetFirstMotion AttachTo)
      (Variables|Default|SetFirstHand%20Mesh HandMesh)
      (Physics|SetSimulatePhysics (Variables|Default|GetSkeletalMesh) false)
      (Transformation|AttachComponentToComponent (Variables|Default|GetSkeletalMesh) (Variables|Default|GetFirstHand%20Mesh) "hand_Socket" "SnapToTarget" "SnapToTarget" "KeepWorld" false))))

(event EventDrop
  (params (HandMesh :type Scene%20Component%20Object%20Reference) (MotionController :type Scene%20Component%20Object%20Reference))
  (if (== MotionController (Variables|Default|GetFirstMotion))
    (Physics|SetSimulatePhysics (Variables|Default|GetSkeletalMesh) true)
    (Transformation|DetachFromComponent (Variables|Default|GetSkeletalMesh) "KeepWorld" "KeepWorld" "KeepWorld" true)
    (Variables|Default|SetFirstMotion 0)
    (Variables|Default|SetSecondMontion 0)
    (else
      (Variables|Default|SetSecondMontion 0)
      (CallFunction|Shoot)
      (Transformation|SetWorldRotation (Variables|Default|GetSkeletalMesh) (Transformation|GetSocketRotation (Variables|Default|GetFirstHand%20Mesh) "hand_Socket") false false))))

(fn ConstructionScript)

(fn GetDistanceHands
  (return (Math|Vector|Distance(Vector) (Transformation|GetWorldLocation (Variables|Default|GetFirstHand%20Mesh)) (Transformation|GetWorldLocation (Variables|Default|GetSecondHand%20Mesh)))))