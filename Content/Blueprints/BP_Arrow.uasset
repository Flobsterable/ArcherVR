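; BP_Arrow is an arrow actor with a projectile launch and stubbed pickup hooks for BP_MotionController.
; Shoot sets projectile speed along local Y, enables query-only sphere collision and flags flight; BeginPlay calls it with zero velocity.
; Pickup, Drop and overlap events are empty.
; Logic for stopping flight, detaching and attaching to a hand mesh, snapping near its socket, is disconnected and never runs.
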(event OnComponentBeginOverlap(Sphere)
  (params (OverlappedComponent :type Primitive%20Component%20Object%20Reference) (OtherActor :type Actor%20Object%20Reference) (OtherComp :type Primitive%20Component%20Object%20Reference) (OtherBodyIndex :type Integer) (bFromSweep :type Boolean) (SweepResult :type Hit%20Result%20Structure%20%28by%20ref%29)))

(event Custom|Shoot
  (params (Velocity :type Float%20%28single-precision%29))
  (bind _projectilemovement (Variables|Default|GetProjectileMovement))
  (Variables|/Script/Engine.ProjectileMovementComponent|SetInitialSpeed _projectilemovement Velocity)
  (bind _output_get (Variables|/Script/Engine.ProjectileMovementComponent|SetMaxSpeed _projectilemovement Velocity))
  (Game|Components|ProjectileMovement|SetVelocityinLocalSpace _projectilemovement (Math|Vector|MakeVector 0.0 _output_get 0.0))
  (Collision|SetCollisionEnabled (Variables|Default|GetSphere) "QueryOnly")
  (Variables|Default|SetFlight? true))

(event EventBeginPlay
  (CallFunction|Shoot 0.0))

(event EventPickup
  (params (AttachTo :type Scene%20Component%20Object%20Reference) (HandMesh :type Scene%20Component%20Object%20Reference)))

(event EventDrop
  (params (HandMesh :type Scene%20Component%20Object%20Reference) (MotionController :type Scene%20Component%20Object%20Reference)))

(fn ConstructionScript)